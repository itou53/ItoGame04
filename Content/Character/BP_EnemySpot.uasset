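; BP_EnemySpot is an enemy spawn point that repeatedly spawns BP_Enemy actors on team 1 at its BillboardSpot transform.
; It spawns one enemy on BeginPlay, then runs the SpawnTimer timeline, which spawns another and restarts itself on each finish.
; Timeline updates feed the Percent track to the W_EnemySpot_SpawnTimer widget as a countdown display.
; EndSpawnTimer stops the timeline, halting the loop.
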(event Custom|SpawnEnemy
  (bind _returnvalue (Game|SpawnActorfromClass "/Game/Character/BP_Enemy/BP_Enemy.BP_Enemy_C" (Transformation|GetWorldTransform (Variables|Default|GetBillboard_spot)) "Undefined" "MultiplyWithRoot" 0 0))
  (Variables|/Game/Character/BP_Enemy/BP_Enemy.BP_Enemy_C|SetTeamNumber _returnvalue 1))

(event Custom|EndSpawnTimer
  (bind _percent (Timeline|SpawnTimer Stop)
    (:Update
      (bind _output_get (Variables|Default|SetCurrentPercent _percent))
      (Default|UpdateTimer (.AsW%20Enemy%20Spot%20Spawn%20Timer (Utilities|Casting|CastToW_EnemySpot_SpawnTimer (UserInterface|GetWidget (Variables|Default|GetWidget)))) _output_get))
    (:Finished
      (CallFunction|SpawnEnemy)
      (CallFunction|StartSpawnTimer))))

(event Custom|StartSpawnTimer
  (bind _percent (Timeline|SpawnTimer PlayFromStart)
    (:Update
      (bind _output_get (Variables|Default|SetCurrentPercent _percent))
      (Default|UpdateTimer (.AsW%20Enemy%20Spot%20Spawn%20Timer (Utilities|Casting|CastToW_EnemySpot_SpawnTimer (UserInterface|GetWidget (Variables|Default|GetWidget)))) _output_get))
    (:Finished
      (CallFunction|SpawnEnemy)
      (CallFunction|StartSpawnTimer))))

(event EventBeginPlay
  (CallFunction|SpawnEnemy)
  (CallFunction|StartSpawnTimer))

(fn ConstructionScript)