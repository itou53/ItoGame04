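; Enemy character Blueprint that attacks a given target and can strike a victory pose.
; BeginPlay caches the mesh's ABP_Enemy anim instance, which the events drive through boolean flags.
; Attack runs a macro that pulses IsAttacking for half a second, then applies fixed damage to the target with no range or hit check.
; DoVictoryPose sets IsVictory on the anim instance.
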(event Custom|Attack
  (params (TargetActor :type Actor%20Object%20Reference))
  (Utilities|MacroPlayAttackAnimation)
  (Game|Damage|ApplyDamage TargetActor 1e+02 0 0))

(event Custom|DoVictoryPose
  (Variables|/Game/Character/ABP_Enemy.ABP_Enemy_C|SetIsVictory (Variables|Default|GetAs%20ABP%20Enemy) true))

(event EventBeginPlay
  (bind _asabp_enemy (Utilities|Casting|CastToABP_Enemy (Components|SkeletalMesh|GetAnimInstance (Variables|Character|GetMesh))))
  (Variables|Default|SetAs%20ABP%20Enemy _asabp_enemy)
  (Utilities|FlowControl|Delay 1.0))

(fn ConstructionScript)