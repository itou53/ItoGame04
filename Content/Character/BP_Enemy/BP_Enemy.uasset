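; BP_Enemy is an enemy character that attacks targets, takes damage, dies and can strike a victory pose.
; Its construction script loads stats from the first row of DataTable_EnemyStatus and sets walk speed.
; Attack deals damage immediately while a macro raises the attacking flag for half a second.
; Incoming damage reduces health, and attack, death and victory states are written directly to ABP_Enemy flags.
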(event Custom|Attack
  (params (TargetActor :type Actor%20Object%20Reference))
  (Utilities|FlowControl|Sequence
    (:then_0
      (Utilities|MacroPlayAttackAnimation))
    (:then_1
      (Game|Damage|ApplyDamage TargetActor (.Attack (Utilities|Struct|BreakBP_EnemyStatus (Variables|Default|GetEnemyStatus))) 0 0))))

(event Custom|DoVictoryPose
  (Variables|/Game/Character/BP_Enemy/ABP_Enemy.ABP_Enemy_C|SetIsVictory (Variables|Default|GetAs%20ABP%20Enemy) true))

(event EventBeginPlay
  (bind _asabp_enemy (Utilities|Casting|CastToABP_Enemy (Components|SkeletalMesh|GetAnimInstance (Variables|Character|GetMesh))))
  (Variables|Default|SetAs%20ABP%20Enemy _asabp_enemy)
  (Utilities|FlowControl|Delay 1.0))

(event Game|Damage|EventAnyDamage
  (params (Damage :type Float%20%28single-precision%29) (DamageType :type Damage%20Type%20Object%20Reference) (InstigatedBy :type Controller%20Object%20Reference) (DamageCauser :type Actor%20Object%20Reference))
  (bind _output_get (Variables|Default|SetEnemyStatus (Utilities|Struct|MakeBP_EnemyStatus (- (.Health (Utilities|Struct|BreakBP_EnemyStatus (Variables|Default|GetEnemyStatus))) Damage) (.Attack (Utilities|Struct|BreakBP_EnemyStatus (Variables|Default|GetEnemyStatus))) (.MoveSpeed (Utilities|Struct|BreakBP_EnemyStatus (Variables|Default|GetEnemyStatus))) (.AttackRange (Utilities|Struct|BreakBP_EnemyStatus (Variables|Default|GetEnemyStatus))) (.AttackSpeed (Utilities|Struct|BreakBP_EnemyStatus (Variables|Default|GetEnemyStatus))))))
  (if (<= (.Health (Utilities|Struct|BreakBP_EnemyStatus _output_get)) 0.0)
    (Variables|/Game/Character/BP_Enemy/ABP_Enemy.ABP_Enemy_C|SetIsDead (Variables|Default|GetAs%20ABP%20Enemy) true)
    (Variables|Default|SetIsDead true)))

(fn ConstructionScript
  (bind _outrownames (DataTable|GetDataTableRowNames "/Game/Character/BP_Enemy/DataTable_EnemyStatus.DataTable_EnemyStatus"))
  (bind _returnvalue (Utilities|GetDataTableRow "/Game/Character/BP_Enemy/DataTable_EnemyStatus.DataTable_EnemyStatus" (Utilities|Array|Get(acopy) _outrownames))
    (:then
      (bind _output_get (Variables|Default|SetEnemyStatus _returnvalue))
      (Variables|/Script/Engine.CharacterMovementComponent|SetMaxWalkSpeed (Variables|Character|GetCharacterMovement) (.MoveSpeed (Utilities|Struct|BreakBP_EnemyStatus _output_get))))))